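; BP_BaseInteract is a base interactable item with a mesh and a sphere trigger that players can register with.
; The construction script applies configurable mesh scale and trigger radius.
; When a BP_Player enters or leaves the sphere, the item registers or unregisters itself with that player.
; SetOutline toggles the mesh's custom depth rendering for highlighting.
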(event `self.Trigger.OnComponentBeginOverlap`
  (params (OverlappedComponent :type "PrimitiveComponent Object Reference") (OtherActor :type "Actor Object Reference") (OtherComp :type "PrimitiveComponent Object Reference") (OtherBodyIndex :type Integer) (bFromSweep :type Boolean) (SweepResult :type "HitResult Structure (by ref)"))
  (bind _asbp_player (cast `/Game/Player/BluePrint/BP_Player` OtherActor))
  (message `/Game/Item/Data/InteractData/BPI_Interact.RegisterInteractable` _asbp_player self))

(event `self.Trigger.OnComponentEndOverlap`
  (params (OverlappedComponent :type "PrimitiveComponent Object Reference") (OtherActor :type "Actor Object Reference") (OtherComp :type "PrimitiveComponent Object Reference") (OtherBodyIndex :type Integer))
  (bind _asbp_player (cast `/Game/Player/BluePrint/BP_Player` OtherActor))
  (message `/Game/Item/Data/InteractData/BPI_Interact.UnRegisterInteractable` _asbp_player self))

(fn `SetOutline`
  (params (`Outligth?` :type Boolean))
  (`PrimitiveComponent.SetRenderCustomDepth` (`self.SM_Item`) `Outligth?`))

(fn `UserConstructionScript`
  (`SceneComponent.SetWorldScale3D` (`self.SM_Item`) (`self.Mesh Scale`))
  (`SphereComponent.SetSphereRadius` (`self.Trigger`) (`self.Trigger Scale`) true))