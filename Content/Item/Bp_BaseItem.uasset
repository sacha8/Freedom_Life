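; Bp_BaseItem is a base pickup item that a character collects into an inventory.
; Its construction script rebuilds the ItemInfo struct, keeping the other fields and filling in the item's own class.
; On Interaction, it checks that the character has inventory space, passes ItemInfo to the character's PickUpMessage and destroys itself.
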(event `/Game/Item/Data/InteractData/BPI_Interact.Interaction`
  (params (Character :type "/Game/Player/BluePrint/BP_Player Object Reference"))
  (if (`/Game/Player/BluePrint/BP_Player.HasSpaceInventory` Character)
    (message `/Game/Item/Data/InteractData/BPI_Interact.PickUp` Character (`self.ItemInfo`))
    (`self.K2_DestroyActor`)))

(fn `UserConstructionScript`
  (bind (_iteminfo_itemtype _iteminfo_equipementslot _iteminfo_itemname _iteminfo_itemdescription _iteminfo_itemicon _iteminfo_itemclass _iteminfo_itemindex) (break `/Game/Item/Data/S_ItemInfo` (`self.ItemInfo`)))
  (`parent.UserConstructionScript`)
  (set `self.ItemInfo` (make `/Game/Item/Data/S_ItemInfo` _iteminfo_itemtype _iteminfo_equipementslot _iteminfo_itemname _iteminfo_itemdescription _iteminfo_itemicon (`GameplayStatics.GetObjectClass` self) _iteminfo_itemindex)))