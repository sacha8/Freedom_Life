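; GM_Player, likely a game mode given its prefix, runs a looping time-of-day clock.
; Tick adds delta time scaled by GameSecondsInFlealSeconds to TimeOfDaySeconde and wraps it by modulo once it exceeds SecondsInDay.
; BeginPlay stores the first BP_Player actor found in a variable named SkySphere, which nothing else in the graph uses.
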(event `self.ReceiveBeginPlay`
  (bind _outactors (`GameplayStatics.GetAllActorsOfClass` "/Game/Player/BluePrint/BP_Player.BP_Player_C"))
  (set `self.SkySphere` (`|GetArrayItem` _outactors)))

(event `self.ReceiveTick`
  (params (DeltaSeconds :type "Float (single-precision)"))
  (bind _output_get (set `self.TimeOfDay [Seconde]` (+ (`self.TimeOfDay [Seconde]`) (* DeltaSeconds (`self.GameSecondsInFlealSeconds`)))))
  (if (> _output_get (`self.SecondsInDay`))
    (set `self.TimeOfDay [Seconde]` (mod (`self.TimeOfDay [Seconde]`) (`self.SecondsInDay`)))))

(fn `UserConstructionScript`)