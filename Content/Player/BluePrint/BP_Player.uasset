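; Player character Blueprint with movement, sprinting drained by a looping stamina timer, damage intake, item pickup, inventory and equipment.
; Each tick it outlines an overlapping interactable from a registered list, which the pickup input messages.
; Using clothes or weapons swaps the slot's item back to inventory, spawns the actor on a mesh socket and notifies CharaLiveRef.
; Inventory and equipment widgets rebuild on changes, and dropped items respawn with physics.
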(event `/Game/Item/Data/BPI_Equipement.DropItem`
  (params (ItemInfo :type "/Game/Item/Data/S_ItemInfo Structure"))
  (`self.RemoveFromInventory` ItemInfo)
  (`self.RefreshInventory`)
  (`self.SpawnDroppedItem` ItemInfo))

(event `/Game/Item/Data/BPI_CharaLivePreview.PassReference`
  (params (CharaRef :type "/Game/Player/Inventaire/LivePreview/BP_LivePreview Object Reference"))
  (set `self.CharaLiveRef` CharaRef))

(event `/Game/Item/Data/BPI_Equipement.UseItem`
  (params (ItemInfo :type "/Game/Item/Data/S_ItemInfo Structure"))
  (`self.RemoveFromInventory` ItemInfo)
  (switch `/Game/Item/Data/E_ItemType` (`.ItemType_12_A1B964AC4818CCCBD985D0B3C26A73D1` (break `/Game/Item/Data/S_ItemInfo` ItemInfo))
    (:`NewEnumerator1`
      _)
    (:`NewEnumerator3`
      _))
  (`self.UpdateEquipementSlot` ItemInfo)
  (`self.AttachEquipement` ItemInfo)
  (message `/Game/Item/Data/BPI_CharaLivePreview.EquipItem` (`self.CharaLiveRef`) ItemInfo))

(event `/Game/Item/Data/BPI_Equipement.UnUseItem`
  (params (ItemInfo :type "/Game/Item/Data/S_ItemInfo Structure"))
  (`self.RemoveFromEquipement` ItemInfo)
  (`self.AddToInventory` ItemInfo)
  (`self.RefreshEquipement`)
  (`self.UnAttachEquipement` ItemInfo)
  (message `/Game/Item/Data/BPI_CharaLivePreview.UnEquipItem` (`self.CharaLiveRef`) ItemInfo))

(event `self.ReceiveTick`
  (params (DeltaSeconds :type "Float (single-precision)"))
  (`|ExecutionSequence`
    (:`then_0`
      (`self.UpdateBestInteractable`))))

(event `InputAction|OpenInventory`
  (params (Key :type "Key Structure"))
  (bind _returnvalue (`GameplayStatics.GetPlayerController` 0))
  (bind _returnvalue_2 (`GameplayStatics.GetPlayerController` 0))
  ;[1 1 1] Nodes
  (:`Pressed`
    (if (`self.IsInventoryOpen`)
      (`Widget.RemoveFromParent` (`self.UI_InventoryRef`))
      (if (`self.IsEquipement`)
        (set `self.IsInventoryOpen` false)
        (else
          (`WidgetBlueprintLibrary.SetInputMode_GameOnly` _returnvalue)
          (set `PlayerController.bShowMouseCursor` false _returnvalue)
          (set `self.IsInventoryOpen` false)))
      (else
        (bind _returnvalue_3 (`|CreateWidget` "/Game/Player/Inventaire/UI_Inventory.UI_Inventory_C"))
        (bind _output_get (set `self.UI_InventoryRef` _returnvalue_3))
        (`UserWidget.AddToViewport` _output_get 0)
        (`WidgetBlueprintLibrary.SetInputMode_GameAndUIEx` _returnvalue_2 _output_get)
        (set `PlayerController.bShowMouseCursor` true _returnvalue_2)
        (set `self.IsInventoryOpen` true)))))

(event `InputAction|OpenEquipement`
  (params (Key :type "Key Structure"))
  (bind _returnvalue (`GameplayStatics.GetPlayerController` 0))
  ;[1 1 1] Nodes
  (:`Pressed`
    (if (`self.IsEquipement`)
      (`Widget.RemoveFromParent` (`self.UI_EquipementRef`))
      (if (`self.IsInventoryOpen`)
        (set `self.IsEquipement` false)
        (else
          (`WidgetBlueprintLibrary.SetInputMode_GameOnly` _returnvalue)
          (set `PlayerController.bShowMouseCursor` false _returnvalue)
          (set `self.IsEquipement` false)))
      (else
        (bind _returnvalue_2 (`|CreateWidget` "/Game/Player/Inventaire/UI_Equipement.UI_Equipement_C"))
        (bind _output_get (set `self.UI_EquipementRef` _returnvalue_2))
        (`UserWidget.AddToViewport` _output_get 0)
        (`WidgetBlueprintLibrary.SetInputMode_GameAndUIEx` _returnvalue _output_get)
        (set `PlayerController.bShowMouseCursor` true _returnvalue)
        (set `self.IsEquipement` true)))))

(event `InputAction|PickUpItem`
  (params (Key :type "Key Structure"))
  (bind _iteminteract (`self.ItemInteract`))
  ;[1 1 1] Nodes
  (:`Pressed`
    (`/Engine/EditorBlueprintResources/StandardMacros.IsValid` _iteminteract
      (:`Is Valid`
        (message `/Game/Item/Data/InteractData/BPI_Interact.Interaction` _iteminteract self)))))

(event `/Game/Item/Data/InteractData/BPI_Interact.PickUp`
  (params (ItemInfo :type "/Game/Item/Data/S_ItemInfo Structure"))
  ;[1 1 1] Nodes
  (`self.AddToInventory` ItemInfo))

(event `/Game/Item/Data/InteractData/BPI_Interact.RegisterInteractable`
  (params (Interact :type "/Game/Item/Data/InteractData/BP_BaseInteract Object Reference"))
  ;[1 1 1] Nodes
  (`self.HandleRegisterInteract` Interact))

(event `/Game/Item/Data/InteractData/BPI_Interact.UnRegisterInteractable`
  (params (Interact :type "/Game/Item/Data/InteractData/BP_BaseInteract Object Reference"))
  ;[1 1 1] Nodes
  (`self.HandleUnRegisterInteract` Interact))

(event `InputAxis|MoveForward`
  (params (AxisValue :type "Float (single-precision)"))
  ;[1 1 1] Nodes
  (`self.AddMovementInput` (`KismetMathLibrary.GetForwardVector` (`KismetMathLibrary.MakeRotator` 0.0 0.0 (.yaw (`self.GetControlRotation`)))) AxisValue))

(event `InputAxis|LookUp`
  (params (AxisValue :type "Float (single-precision)"))
  ;[1 1 1] Nodes
  (`self.AddControllerPitchInput` self AxisValue))

(event `InputAction|Jump`
  (params (Key :type "Key Structure"))
  ;[1 1 1] Nodes
  (:`Pressed`
    (`self.Jump`))
  (:`Released`
    (`self.StopJumping`)))

(event `InputAxis|MoveRight`
  (params (AxisValue :type "Float (single-precision)"))
  ;[1 1 1] Nodes
  (`self.AddMovementInput` (`KismetMathLibrary.GetRightVector` (`KismetMathLibrary.MakeRotator` 0.0 0.0 (.yaw (`self.GetControlRotation`)))) AxisValue))

(event `InputAxis|LookRight`
  (params (AxisValue :type "Float (single-precision)"))
  ;[1 1 1] Nodes
  (`self.AddControllerYawInput` self AxisValue))

(event `InputAction|Sprint`
  (params (Key :type "Key Structure"))
  (bind _charactermovement (`self.CharacterMovement`))
  ;[1 1 1] Nodes
  (:`Pressed`
    (set `CharacterMovementComponent.MaxWalkSpeed` 600.0 _charactermovement)
    (`GameplayStatics.PlayWorldCameraShake` null)
    (set `self.Timer` 0.1)
    (bind _returnvalue (`KismetSystemLibrary.K2_SetTimer` null "Stamina" (`self.Timer`) true :!label _label))
    (set `self.TimerStamina` _returnvalue))
  (:`Released`
    (set `CharacterMovementComponent.MaxWalkSpeed` 180.0 _charactermovement)
    (goto _label)))

(event `self.ReceiveAnyDamage`
  (params (Damage :type "Float (single-precision)") (DamageType :type "DamageType Object Reference") (InstigatedBy :type "Controller Object Reference") (DamageCauser :type "Actor Object Reference"))
  ;[1 1 1] Nodes
  (set `self.CurrentLife` (- (`self.CurrentLife`) Damage)))

(fn `AddToEquipement`
  (params (ItemInfo :type "/Game/Item/Data/S_ItemInfo Structure (by ref)"))
  (bind _ui_equipementref (`self.UI_EquipementRef`))
  (`KismetArrayLibrary.Array_Add` (`self.Equipement`) ItemInfo)
  (`/Engine/EditorBlueprintResources/StandardMacros.IsValid` _ui_equipementref
    (:`Is Valid`
      (`/Game/Player/Inventaire/UI_Equipement.CreateEquipement` _ui_equipementref))))

(fn `AddToInventory`
  (params (ItemInfo :type "/Game/Item/Data/S_ItemInfo Structure (by ref)"))
  (bind _ui_inventoryref (`self.UI_InventoryRef`))
  (`KismetArrayLibrary.Array_Add` (`self.Inventory`) ItemInfo)
  (`/Engine/EditorBlueprintResources/StandardMacros.IsValid` _ui_inventoryref
    (:`Is Valid`
      (`PanelWidget.ClearChildren` (`/Game/Player/Inventaire/UI_Inventory.InventoryPanel` _ui_inventoryref))
      (`/Game/Player/Inventaire/UI_Inventory.CreateInventory` _ui_inventoryref))))

(fn `AttachEquipement`
  (params (`item Info` :type "/Game/Item/Data/S_ItemInfo Structure"))
  (bind ((`EquipementSlot_20_97FFB28141FA50374491FBABAC252A3D` _equipementslot) (`ItemClass_16_F1B555F24A4B69AE0A2BA2BC3542EAEC` _itemclass)) (break `/Game/Item/Data/S_ItemInfo` `item Info`))
  (switch `/Game/Item/Data/E_EquipementSlot` _equipementslot
    (:`NewEnumerator1`
      (`/Engine/EditorBlueprintResources/StandardMacros.IsValid` (`self.HeadItem`)
        (:`Is Valid`
          (`self.K2_DestroyActor` (`self.HeadItem`)))
        (:`Is Not Valid`
          _))
      (bind _returnvalue (`|SpawnActorFromClass` _itemclass (`self.GetTransform`) "AlwaysSpawn" "OverrideRootScale" null null))
      (bind _output_get (set `self.HeadItem` _returnvalue))
      (bind _asbp_base_clothes (cast `/Game/Item/Clothes/Bp_BaseClothes` _output_get))
      (`self.K2_AttachToComponent` _asbp_base_clothes (`self.Mesh`) (`.SocketName_2_37CC62534CE280118F339CA1F83C393B` (break `/Game/Item/Clothes/S_ClothesSocket` (`/Game/Item/Clothes/Bp_BaseClothes.ClothesInfos` _asbp_base_clothes))) "SnapToTarget" "SnapToTarget" "SnapToTarget" true)
      (`self.SetActorEnableCollision` _asbp_base_clothes false)
      (`PrimitiveComponent.SetSimulatePhysics` (`/Game/Item/Data/InteractData/BP_BaseInteract.SM_Item` _asbp_base_clothes) false))
    (:`NewEnumerator2`
      (`/Engine/EditorBlueprintResources/StandardMacros.IsValid` (`self.TorsoItem`)
        (:`Is Valid`
          (`self.K2_DestroyActor` (`self.TorsoItem`)))
        (:`Is Not Valid`
          _))
      (bind _returnvalue_2 (`|SpawnActorFromClass` _itemclass (`self.GetTransform`) "AlwaysSpawn" "OverrideRootScale" null null))
      (bind _output_get_2 (set `self.TorsoItem` _returnvalue_2))
      (bind _asbp_base_clothes_2 (cast `/Game/Item/Clothes/Bp_BaseClothes` _output_get_2))
      (`self.K2_AttachToComponent` _asbp_base_clothes_2 (`self.Mesh`) (`.SocketName_2_37CC62534CE280118F339CA1F83C393B` (break `/Game/Item/Clothes/S_ClothesSocket` (`/Game/Item/Clothes/Bp_BaseClothes.ClothesInfos` _asbp_base_clothes_2))) "SnapToTarget" "SnapToTarget" "SnapToTarget" true)
      (`self.SetActorEnableCollision` _asbp_base_clothes_2 false)
      (`PrimitiveComponent.SetSimulatePhysics` (`/Game/Item/Data/InteractData/BP_BaseInteract.SM_Item` _asbp_base_clothes_2) false))
    (:`NewEnumerator7`
      (`/Engine/EditorBlueprintResources/StandardMacros.IsValid` (`self.HandsItem`)
        (:`Is Valid`
          (`self.K2_DestroyActor` (`self.HandsItem`)))
        (:`Is Not Valid`
          _))
      (bind _returnvalue_3 (`|SpawnActorFromClass` _itemclass (`self.GetTransform`) "AlwaysSpawn" "OverrideRootScale" null null))
      (bind _output_get_3 (set `self.HandsItem` _returnvalue_3))
      (bind _asbp_base_clothes_3 (cast `/Game/Item/Clothes/Bp_BaseClothes` _output_get_3))
      (`self.K2_AttachToComponent` _asbp_base_clothes_3 (`self.Mesh`) (`.SocketName_2_37CC62534CE280118F339CA1F83C393B` (break `/Game/Item/Clothes/S_ClothesSocket` (`/Game/Item/Clothes/Bp_BaseClothes.ClothesInfos` _asbp_base_clothes_3))) "SnapToTarget" "SnapToTarget" "SnapToTarget" true)
      (`self.SetActorEnableCollision` _asbp_base_clothes_3 false)
      (`PrimitiveComponent.SetSimulatePhysics` (`/Game/Item/Data/InteractData/BP_BaseInteract.SM_Item` _asbp_base_clothes_3) false))
    (:`NewEnumerator3`
      (`/Engine/EditorBlueprintResources/StandardMacros.IsValid` (`self.RightHandItem`)
        (:`Is Valid`
          (`self.K2_DestroyActor` (`self.RightHandItem`)))
        (:`Is Not Valid`
          _))
      (bind _returnvalue_4 (`|SpawnActorFromClass` _itemclass (`self.GetTransform`) "AlwaysSpawn" "OverrideRootScale" null null))
      (bind _output_get_4 (set `self.RightHandItem` _returnvalue_4))
      (bind _asbp_base_weapon (cast `/Game/Item/Weapon/BP_BaseWeapon` _output_get_4))
      (`self.K2_AttachToComponent` _asbp_base_weapon (`self.Mesh`) (`.RightHand_3_5308C62E4819B7AD27264E8335C5E7E6` (break `/Game/Item/Weapon/S_WeaponInfo` (`/Game/Item/Weapon/BP_BaseWeapon.WeaponeInfo` _asbp_base_weapon))) "SnapToTarget" "SnapToTarget" "SnapToTarget" true)
      (`self.SetActorEnableCollision` _asbp_base_weapon false)
      (`PrimitiveComponent.SetSimulatePhysics` (`/Game/Item/Data/InteractData/BP_BaseInteract.SM_Item` _asbp_base_weapon) false))
    (:`NewEnumerator4`
      (`/Engine/EditorBlueprintResources/StandardMacros.IsValid` (`self.LeftHandItem`)
        (:`Is Valid`
          (`self.K2_DestroyActor` (`self.LeftHandItem`)))
        (:`Is Not Valid`
          _))
      (bind _returnvalue_5 (`|SpawnActorFromClass` _itemclass (`self.GetTransform`) "AlwaysSpawn" "OverrideRootScale" null null))
      (bind _output_get_5 (set `self.LeftHandItem` _returnvalue_5))
      (bind _asbp_base_weapon_2 (cast `/Game/Item/Weapon/BP_BaseWeapon` _output_get_5))
      (`self.K2_AttachToComponent` _asbp_base_weapon_2 (`self.Mesh`) (`.Lefthand_5_A458576C4A75C88B3C79F282D7BEF06D` (break `/Game/Item/Weapon/S_WeaponInfo` (`/Game/Item/Weapon/BP_BaseWeapon.WeaponeInfo` _asbp_base_weapon_2))) "SnapToTarget" "SnapToTarget" "KeepRelative" true)
      (`self.SetActorEnableCollision` _asbp_base_weapon_2 false)
      (`PrimitiveComponent.SetSimulatePhysics` (`/Game/Item/Data/InteractData/BP_BaseInteract.SM_Item` _asbp_base_weapon_2) false))
    (:`NewEnumerator5`
      (`/Engine/EditorBlueprintResources/StandardMacros.IsValid` (`self.LegsItem`)
        (:`Is Valid`
          (`self.K2_DestroyActor` (`self.LegsItem`)))
        (:`Is Not Valid`
          _))
      (bind _returnvalue_6 (`|SpawnActorFromClass` _itemclass (`self.GetTransform`) "AlwaysSpawn" "OverrideRootScale" null null))
      (bind _output_get_6 (set `self.LegsItem` _returnvalue_6))
      (bind _asbp_base_clothes_4 (cast `/Game/Item/Clothes/Bp_BaseClothes` _output_get_6))
      (`self.K2_AttachToComponent` _asbp_base_clothes_4 (`self.Mesh`) (`.SocketName_2_37CC62534CE280118F339CA1F83C393B` (break `/Game/Item/Clothes/S_ClothesSocket` (`/Game/Item/Clothes/Bp_BaseClothes.ClothesInfos` _asbp_base_clothes_4))) "SnapToTarget" "SnapToTarget" "SnapToTarget" true)
      (`self.SetActorEnableCollision` _asbp_base_clothes_4 false)
      (`PrimitiveComponent.SetSimulatePhysics` (`/Game/Item/Data/InteractData/BP_BaseInteract.SM_Item` _asbp_base_clothes_4) false))))

(fn `GetBestInteractable`
  (locals (L_InteractVar :type "/Game/Item/Data/InteractData/S_InteractVariables Structure"))
  (bind _l_interactvar_interactable (break `/Game/Item/Data/InteractData/S_InteractVariables` (`local.L_InteractVar`)))
  (set `local.L_InteractVar` (make `/Game/Item/Data/InteractData/S_InteractVariables` null))
  (for _array_element (`self.Interactables`)
    (if (`PrimitiveComponent.IsOverlappingComponent` (`/Game/Item/Data/InteractData/BP_BaseInteract.Trigger` _array_element) (`self.CapsuleComponent`))
      (set `local.L_InteractVar` (make `/Game/Item/Data/InteractData/S_InteractVariables` _array_element))))
  (`/Engine/EditorBlueprintResources/StandardMacros.IsValid` _l_interactvar_interactable
    (:`Is Valid`
      (`self.SetBestInteractable` _l_interactvar_interactable))
    (:`Is Not Valid`
      (`self.SetBestInteractable` null))))

(fn `HandleRegisterInteract`
  (params (Interactable :type "/Game/Item/Data/InteractData/BP_BaseInteract Object Reference (by ref)"))
  (`KismetArrayLibrary.Array_AddUnique` (`self.Interactables`) Interactable))

(fn `HandleUnRegisterInteract`
  (params (Interactable :type "/Game/Item/Data/InteractData/BP_BaseInteract Object Reference (by ref)"))
  (`KismetArrayLibrary.Array_RemoveItem` (`self.Interactables`) Interactable))

(fn `HasSpaceInventory`
  (returns (ReturnValue :type Boolean))
  (return (< (`KismetArrayLibrary.Array_Length` (`self.Inventory`)) (`self.InventorySize`))))

(fn `RefreshEquipement`
  (`/Game/Player/Inventaire/UI_Equipement.CreateEquipement` (`self.UI_EquipementRef`)))

(fn `RefreshInventory`
  (bind _ui_inventoryref (`self.UI_InventoryRef`))
  (`/Engine/EditorBlueprintResources/StandardMacros.IsValid` _ui_inventoryref
    (:`Is Valid`
      (`PanelWidget.ClearChildren` (`/Game/Player/Inventaire/UI_Inventory.InventoryPanel` _ui_inventoryref))
      (`/Game/Player/Inventaire/UI_Inventory.CreateInventory` _ui_inventoryref))))

(fn `RemoveFromEquipement`
  (params (ItemInfo :type "/Game/Item/Data/S_ItemInfo Structure"))
  (`KismetArrayLibrary.Array_Remove` (`self.Equipement`) (`.ItemIndex_17_118FD7EF4BCDA1B432F2E48D473EB554` (break `/Game/Item/Data/S_ItemInfo` ItemInfo))))

(fn `RemoveFromInventory`
  (params (ItemInfo :type "/Game/Item/Data/S_ItemInfo Structure"))
  (`KismetArrayLibrary.Array_Remove` (`self.Inventory`) (`.ItemIndex_17_118FD7EF4BCDA1B432F2E48D473EB554` (break `/Game/Item/Data/S_ItemInfo` ItemInfo))))

(fn `SetBestInteractable`
  (params (Interactable :type "/Game/Item/Data/InteractData/BP_BaseInteract Object Reference"))
  (`/Engine/EditorBlueprintResources/StandardMacros.IsValid` Interactable
    (:`Is Valid`
      (if (!= Interactable (`self.ItemInteract`))
        (bind _iteminteract (`self.ItemInteract`)
          (:`then`
            (`/Game/Item/Data/InteractData/BP_BaseInteract.SetOutline` _iteminteract false))
          (:`else`
            _)))
      (bind _output_get (set `self.ItemInteract` Interactable))
      (`/Game/Item/Data/InteractData/BP_BaseInteract.SetOutline` _output_get true))
    (:`Is Not Valid`
      (bind _iteminteract_2 (`self.ItemInteract`)
        (:`then`
          (`/Game/Item/Data/InteractData/BP_BaseInteract.SetOutline` _iteminteract_2 false)
          (set `self.ItemInteract` null))
        (:`else`)))))

(fn `SpawnDroppedItem`
  (params (ItemInfo :type "/Game/Item/Data/S_ItemInfo Structure"))
  (bind _spawnlocation (`self.SpawnLocation`))
  (bind _returnvalue (`|SpawnActorFromClass` (`.ItemClass_16_F1B555F24A4B69AE0A2BA2BC3542EAEC` (break `/Game/Item/Data/S_ItemInfo` ItemInfo)) (`KismetMathLibrary.MakeTransform` (+ (`SceneComponent.K2_GetComponentLocation` _spawnlocation) (* (`SceneComponent.GetForwardVector` _spawnlocation) 300.0))) "AlwaysSpawn" "OverrideRootScale" null null))
  (`self.SetActorEnableCollision` _returnvalue true)
  (`PrimitiveComponent.SetSimulatePhysics` (`/Game/Item/Data/InteractData/BP_BaseInteract.SM_Item` _returnvalue) true))

(fn `Stamina`
  (if (`MovementComponent.IsExceedingMaxSpeed` (`self.CharacterMovement`) 300.0)
    (if (> (`self.CurrentStamina`) 0.0)
      (set `self.CurrentStamina` (- (`self.CurrentStamina`) 1.5))
      (else
        (set `CharacterMovementComponent.MaxWalkSpeed` 300.0 (`self.CharacterMovement`))))
    (elif (< (`self.CurrentStamina`) (`self.CurrentStaminaMax`))
      (set `self.CurrentStamina` (+ (`self.CurrentStamina`) 1.0))
      (else
        (`KismetSystemLibrary.K2_PauseTimerHandle` (`self.TimerStamina`))))))

(fn `UnAttachEquipement`
  (params (ItemInfo :type "/Game/Item/Data/S_ItemInfo Structure"))
  (switch `/Game/Item/Data/E_EquipementSlot` (`.EquipementSlot_20_97FFB28141FA50374491FBABAC252A3D` (break `/Game/Item/Data/S_ItemInfo` ItemInfo))
    (:`NewEnumerator1`
      (`self.K2_DestroyActor` (`self.HeadItem`)))
    (:`NewEnumerator2`
      (`self.K2_DestroyActor` (`self.TorsoItem`)))
    (:`NewEnumerator7`
      (`self.K2_DestroyActor` (`self.HandsItem`)))
    (:`NewEnumerator3`
      (`self.K2_DestroyActor` (`self.RightHandItem`)))
    (:`NewEnumerator4`
      (`self.K2_DestroyActor` (`self.LeftHandItem`)))
    (:`NewEnumerator5`
      (`self.K2_DestroyActor` (`self.LegsItem`)))))

(fn `UpdateBestInteractable`
  (if (> (`KismetArrayLibrary.Array_Length` (`self.Interactables`)) 0)
    (`self.GetBestInteractable`)
    (else
      (`self.SetBestInteractable` null))))

(fn `UpdateEquipementSlot`
  (params (ItemInfo :type "/Game/Item/Data/S_ItemInfo Structure"))
  (bind _ui_equipementref (`self.UI_EquipementRef`))
  (bind _ui_equipementref_2 (`self.UI_EquipementRef`))
  (bind _ui_equipementref_3 (`self.UI_EquipementRef`))
  (bind _ui_equipementref_4 (`self.UI_EquipementRef`))
  (bind _ui_equipementref_5 (`self.UI_EquipementRef`))
  (bind _ui_equipementref_6 (`self.UI_EquipementRef`))
  (bind _iteminfo (`/Game/Player/Inventaire/UI_EquipementSlot.ItemInfo` (`/Game/Player/Inventaire/UI_Equipement.HandSlot` _ui_equipementref_2)))
  (bind _iteminfo_2 (`/Game/Player/Inventaire/UI_EquipementSlot.ItemInfo` (`/Game/Player/Inventaire/UI_Equipement.RightHandSlot` _ui_equipementref_3)))
  (bind _iteminfo_3 (`/Game/Player/Inventaire/UI_EquipementSlot.ItemInfo` (`/Game/Player/Inventaire/UI_Equipement.LeftHandSlot` _ui_equipementref_4)))
  (bind _iteminfo_4 (`/Game/Player/Inventaire/UI_EquipementSlot.ItemInfo` (`/Game/Player/Inventaire/UI_Equipement.LegsSlot` _ui_equipementref_5)))
  (bind _iteminfo_5 (`/Game/Player/Inventaire/UI_EquipementSlot.ItemInfo` (`/Game/Player/Inventaire/UI_Equipement.HeadSlot` _ui_equipementref)))
  (bind _iteminfo_6 (`/Game/Player/Inventaire/UI_EquipementSlot.ItemInfo` (`/Game/Player/Inventaire/UI_Equipement.TorsoSlot` _ui_equipementref_6)))
  (switch `/Game/Item/Data/E_EquipementSlot` (`.EquipementSlot_20_97FFB28141FA50374491FBABAC252A3D` (break `/Game/Item/Data/S_ItemInfo` ItemInfo))
    (:`NewEnumerator1`
      (`/Engine/EditorBlueprintResources/StandardMacros.IsValid` _ui_equipementref
        (:`Is Valid`
          (if (== (`.ItemClass_16_F1B555F24A4B69AE0A2BA2BC3542EAEC` (break `/Game/Item/Data/S_ItemInfo` _iteminfo_5)) null)
            (`self.AddToEquipement` ItemInfo :!label _label)
            (`self.RefreshInventory`)
            (else
              (`self.AddToInventory` _iteminfo_5)
              (`self.RemoveFromEquipement` _iteminfo_5)
              (`self.AddToEquipement` ItemInfo))))
        (:`Is Not Valid`
          (goto _label))))
    (:`NewEnumerator2`
      (`/Engine/EditorBlueprintResources/StandardMacros.IsValid` _ui_equipementref_6
        (:`Is Valid`
          (if (== (`.ItemClass_16_F1B555F24A4B69AE0A2BA2BC3542EAEC` (break `/Game/Item/Data/S_ItemInfo` _iteminfo_6)) null)
            (`self.AddToEquipement` ItemInfo :!label _label_2)
            (`self.RefreshInventory`)
            (else
              (`self.AddToInventory` _iteminfo_6)
              (`self.RemoveFromEquipement` _iteminfo_6)
              (`self.AddToEquipement` ItemInfo))))
        (:`Is Not Valid`
          (goto _label_2))))
    (:`NewEnumerator7`
      (`/Engine/EditorBlueprintResources/StandardMacros.IsValid` _ui_equipementref_2
        (:`Is Valid`
          (if (== (`.ItemClass_16_F1B555F24A4B69AE0A2BA2BC3542EAEC` (break `/Game/Item/Data/S_ItemInfo` _iteminfo)) null)
            (`self.AddToEquipement` ItemInfo :!label _label_3)
            (`self.RefreshInventory`)
            (else
              (`self.AddToInventory` _iteminfo)
              (`self.RemoveFromEquipement` _iteminfo)
              (`self.AddToEquipement` ItemInfo))))
        (:`Is Not Valid`
          (goto _label_3))))
    (:`NewEnumerator3`
      (`/Engine/EditorBlueprintResources/StandardMacros.IsValid` _ui_equipementref_3
        (:`Is Valid`
          (if (== (`.ItemClass_16_F1B555F24A4B69AE0A2BA2BC3542EAEC` (break `/Game/Item/Data/S_ItemInfo` _iteminfo_2)) null)
            (`self.AddToEquipement` ItemInfo :!label _label_4)
            (`self.RefreshInventory`)
            (else
              (`self.AddToInventory` _iteminfo_2)
              (`self.RemoveFromEquipement` _iteminfo_2)
              (`self.AddToEquipement` ItemInfo))))
        (:`Is Not Valid`
          (goto _label_4))))
    (:`NewEnumerator4`
      (`/Engine/EditorBlueprintResources/StandardMacros.IsValid` _ui_equipementref_4
        (:`Is Valid`
          (if (== (`.ItemClass_16_F1B555F24A4B69AE0A2BA2BC3542EAEC` (break `/Game/Item/Data/S_ItemInfo` _iteminfo_3)) null)
            (`self.AddToEquipement` ItemInfo :!label _label_5)
            (`self.RefreshInventory`)
            (else
              (`self.AddToInventory` _iteminfo_3)
              (`self.RemoveFromEquipement` _iteminfo_3)
              (`self.AddToEquipement` ItemInfo))))
        (:`Is Not Valid`
          (goto _label_5))))
    (:`NewEnumerator5`
      (`/Engine/EditorBlueprintResources/StandardMacros.IsValid` _ui_equipementref_5
        (:`Is Valid`
          (if (== (`.ItemClass_16_F1B555F24A4B69AE0A2BA2BC3542EAEC` (break `/Game/Item/Data/S_ItemInfo` _iteminfo_4)) null)
            (`self.AddToEquipement` ItemInfo :!label _label_6)
            (`self.RefreshInventory`)
            (else
              (`self.AddToInventory` _iteminfo_4)
              (`self.RemoveFromEquipement` _iteminfo_4)
              (`self.AddToEquipement` ItemInfo))))
        (:`Is Not Valid`
          (goto _label_6))))))

(fn `UserConstructionScript`)