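; Live preview actor for the player inventory that displays equipped items, registering itself with BP_Player on BeginPlay.
; EquipItem replaces whatever occupies the item's slot (head, torso, hands, legs, right or left hand) by spawning its class and attaching it to a socket.
; Clothes and weapons supply their own socket names, and spawned items get collision and physics disabled.
; UnEquipItem destroys the actor held in that slot.
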(event `self.ReceiveBeginPlay`
  (bind _asbp_player (cast `/Game/Player/BluePrint/BP_Player` (`GameplayStatics.GetPlayerCharacter` 0)))
  (message `/Game/Item/Data/BPI_CharaLivePreview.PassReference` _asbp_player self))

(event `/Game/Item/Data/BPI_CharaLivePreview.EquipItem`
  (params (ItemInfo :type "/Game/Item/Data/S_ItemInfo Structure"))
  (`self.AttachEquip` ItemInfo))

(event `/Game/Item/Data/BPI_CharaLivePreview.UnEquipItem`
  (params (ItemInfo :type "/Game/Item/Data/S_ItemInfo Structure"))
  (`self.UnAttachEquip` ItemInfo))

(fn `AttachEquip`
  (params (ItemInfo :type "/Game/Item/Data/S_ItemInfo Structure"))
  (bind ((`EquipementSlot_20_97FFB28141FA50374491FBABAC252A3D` _equipementslot) (`ItemClass_16_F1B555F24A4B69AE0A2BA2BC3542EAEC` _itemclass)) (break `/Game/Item/Data/S_ItemInfo` ItemInfo))
  (switch `/Game/Item/Data/E_EquipementSlot` _equipementslot
    (:`NewEnumerator1`
      (`/Engine/EditorBlueprintResources/StandardMacros.IsValid` (`self.HeadItem`)
        (:`Is Valid`
          (`self.K2_DestroyActor` (`self.HeadItem`)))
        (:`Is Not Valid`
          _))
      (bind _returnvalue (`|SpawnActorFromClass` _itemclass (`self.GetTransform`) "AlwaysSpawn" "OverrideRootScale" null null))
      (bind _output_get (set `self.HeadItem` _returnvalue))
      (bind _asbp_base_clothes (cast `/Game/Item/Clothes/Bp_BaseClothes` _output_get))
      (`self.K2_AttachToComponent` _asbp_base_clothes null (`.SocketName_2_37CC62534CE280118F339CA1F83C393B` (break `/Game/Item/Clothes/S_ClothesSocket` (`/Game/Item/Clothes/Bp_BaseClothes.ClothesInfos` _asbp_base_clothes))) "SnapToTarget" "SnapToTarget" "SnapToTarget" true)
      (`self.SetActorEnableCollision` _asbp_base_clothes false)
      (`PrimitiveComponent.SetSimulatePhysics` (`/Game/Item/Data/InteractData/BP_BaseInteract.SM_Item` _asbp_base_clothes) false))
    (:`NewEnumerator2`
      (`/Engine/EditorBlueprintResources/StandardMacros.IsValid` (`self.TorsoItem`)
        (:`Is Valid`
          (`self.K2_DestroyActor` (`self.TorsoItem`)))
        (:`Is Not Valid`
          _))
      (bind _returnvalue_2 (`|SpawnActorFromClass` _itemclass (`self.GetTransform`) "AlwaysSpawn" "OverrideRootScale" null null))
      (bind _output_get_2 (set `self.TorsoItem` _returnvalue_2))
      (bind _asbp_base_clothes_2 (cast `/Game/Item/Clothes/Bp_BaseClothes` _output_get_2))
      (`self.K2_AttachToComponent` _asbp_base_clothes_2 null (`.SocketName_2_37CC62534CE280118F339CA1F83C393B` (break `/Game/Item/Clothes/S_ClothesSocket` (`/Game/Item/Clothes/Bp_BaseClothes.ClothesInfos` _asbp_base_clothes_2))) "SnapToTarget" "SnapToTarget" "SnapToTarget" true)
      (`self.SetActorEnableCollision` _asbp_base_clothes_2 false)
      (`PrimitiveComponent.SetSimulatePhysics` (`/Game/Item/Data/InteractData/BP_BaseInteract.SM_Item` _asbp_base_clothes_2) false))
    (:`NewEnumerator7`
      (`/Engine/EditorBlueprintResources/StandardMacros.IsValid` (`self.HandsItem`)
        (:`Is Valid`
          (`self.K2_DestroyActor` (`self.HandsItem`)))
        (:`Is Not Valid`
          _))
      (bind _returnvalue_3 (`|SpawnActorFromClass` _itemclass (`self.GetTransform`) "AlwaysSpawn" "OverrideRootScale" null null))
      (bind _output_get_3 (set `self.HandsItem` _returnvalue_3))
      (bind _asbp_base_clothes_3 (cast `/Game/Item/Clothes/Bp_BaseClothes` _output_get_3))
      (`self.K2_AttachToComponent` _asbp_base_clothes_3 null (`.SocketName_2_37CC62534CE280118F339CA1F83C393B` (break `/Game/Item/Clothes/S_ClothesSocket` (`/Game/Item/Clothes/Bp_BaseClothes.ClothesInfos` _asbp_base_clothes_3))) "SnapToTarget" "SnapToTarget" "SnapToTarget" true)
      (`self.SetActorEnableCollision` _asbp_base_clothes_3 false)
      (`PrimitiveComponent.SetSimulatePhysics` (`/Game/Item/Data/InteractData/BP_BaseInteract.SM_Item` _asbp_base_clothes_3) false))
    (:`NewEnumerator3`
      (`/Engine/EditorBlueprintResources/StandardMacros.IsValid` (`self.RightHandItem`)
        (:`Is Valid`
          (`self.K2_DestroyActor` (`self.RightHandItem`)))
        (:`Is Not Valid`
          _))
      (bind _returnvalue_4 (`|SpawnActorFromClass` _itemclass (`self.GetTransform`) "AlwaysSpawn" "OverrideRootScale" null null))
      (bind _output_get_4 (set `self.RightHandItem` _returnvalue_4))
      (bind _asbp_base_weapon (cast `/Game/Item/Weapon/BP_BaseWeapon` _output_get_4))
      (`self.K2_AttachToComponent` _asbp_base_weapon null (`.RightHand_3_5308C62E4819B7AD27264E8335C5E7E6` (break `/Game/Item/Weapon/S_WeaponInfo` (`/Game/Item/Weapon/BP_BaseWeapon.WeaponeInfo` _asbp_base_weapon))) "SnapToTarget" "SnapToTarget" "SnapToTarget" true)
      (`self.SetActorEnableCollision` _asbp_base_weapon false)
      (`PrimitiveComponent.SetSimulatePhysics` (`/Game/Item/Data/InteractData/BP_BaseInteract.SM_Item` _asbp_base_weapon) false))
    (:`NewEnumerator4`
      (`/Engine/EditorBlueprintResources/StandardMacros.IsValid` (`self.LeftHandItem`)
        (:`Is Valid`
          (`self.K2_DestroyActor` (`self.LeftHandItem`)))
        (:`Is Not Valid`
          _))
      (bind _returnvalue_5 (`|SpawnActorFromClass` _itemclass (`self.GetTransform`) "AlwaysSpawn" "OverrideRootScale" null null))
      (bind _output_get_5 (set `self.LeftHandItem` _returnvalue_5))
      (bind _asbp_base_weapon_2 (cast `/Game/Item/Weapon/BP_BaseWeapon` _output_get_5))
      (`self.K2_AttachToComponent` _asbp_base_weapon_2 null (`.Lefthand_5_A458576C4A75C88B3C79F282D7BEF06D` (break `/Game/Item/Weapon/S_WeaponInfo` (`/Game/Item/Weapon/BP_BaseWeapon.WeaponeInfo` _asbp_base_weapon_2))) "SnapToTarget" "SnapToTarget" "KeepRelative" true)
      (`self.SetActorEnableCollision` _asbp_base_weapon_2 false)
      (`PrimitiveComponent.SetSimulatePhysics` (`/Game/Item/Data/InteractData/BP_BaseInteract.SM_Item` _asbp_base_weapon_2) false))
    (:`NewEnumerator5`
      (`/Engine/EditorBlueprintResources/StandardMacros.IsValid` (`self.LegsItem`)
        (:`Is Valid`
          (`self.K2_DestroyActor` (`self.LegsItem`)))
        (:`Is Not Valid`
          _))
      (bind _returnvalue_6 (`|SpawnActorFromClass` _itemclass (`self.GetTransform`) "AlwaysSpawn" "OverrideRootScale" null null))
      (bind _output_get_6 (set `self.LegsItem` _returnvalue_6))
      (bind _asbp_base_clothes_4 (cast `/Game/Item/Clothes/Bp_BaseClothes` _output_get_6))
      (`self.K2_AttachToComponent` _asbp_base_clothes_4 null (`.SocketName_2_37CC62534CE280118F339CA1F83C393B` (break `/Game/Item/Clothes/S_ClothesSocket` (`/Game/Item/Clothes/Bp_BaseClothes.ClothesInfos` _asbp_base_clothes_4))) "SnapToTarget" "SnapToTarget" "SnapToTarget" true)
      (`self.SetActorEnableCollision` _asbp_base_clothes_4 false)
      (`PrimitiveComponent.SetSimulatePhysics` (`/Game/Item/Data/InteractData/BP_BaseInteract.SM_Item` _asbp_base_clothes_4) false))))

(fn `UnAttachEquip`
  (params (ItemInfo :type "/Game/Item/Data/S_ItemInfo Structure"))
  (switch `/Game/Item/Data/E_EquipementSlot` (`.EquipementSlot_20_97FFB28141FA50374491FBABAC252A3D` (break `/Game/Item/Data/S_ItemInfo` ItemInfo))
    (:`NewEnumerator1`
      (`self.K2_DestroyActor` (`self.HeadItem`)))
    (:`NewEnumerator2`
      (`self.K2_DestroyActor` (`self.TorsoItem`)))
    (:`NewEnumerator7`
      (`self.K2_DestroyActor` (`self.HandsItem`)))
    (:`NewEnumerator3`
      (`self.K2_DestroyActor` (`self.RightHandItem`)))
    (:`NewEnumerator4`
      (`self.K2_DestroyActor` (`self.LeftHandItem`)))
    (:`NewEnumerator5`
      (`self.K2_DestroyActor` (`self.LegsItem`)))))

(fn `UserConstructionScript`)